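; BP_Projectile is a projectile that destroys targets it hits and reports each one to the BP_TargetManager.
; On BeginPlay it caches the manager and destroys itself after a ten-second lifetime.
; Sphere hits only count while the manager is running: a BP_Target is destroyed, the manager's CurrentTargetCount is incremented and the projectile destroys itself.
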(event `self.ReceiveBeginPlay`
  (bind _returnvalue (`GameplayStatics.GetActorOfClass` "/Game/BP_TargetManager.BP_TargetManager_C"))
  (set `self.TargetManagerReference` _returnvalue)
  (`KismetSystemLibrary.Delay` 10.0)
  (`self.K2_DestroyActor` :!label _label))

(event `self.Sphere.OnComponentHit`
  (params (HitComponent :type "PrimitiveComponent Object Reference") (OtherActor :type "Actor Object Reference") (OtherComp :type "PrimitiveComponent Object Reference") (NormalImpulse :type "Vector Structure") (Hit :type "HitResult Structure (by ref)"))
  (bind _targetmanagerreference (`self.TargetManagerReference`))
  (if (`/Game/BP_TargetManager.IsRunning` _targetmanagerreference)
    (bind _asbp_target (cast `/Game/BP_Target` OtherActor))
    (`self.K2_DestroyActor` _asbp_target)
    (set `/Game/BP_TargetManager.CurrentTargetCount` (+ (`/Game/BP_TargetManager.CurrentTargetCount` _targetmanagerreference) 1) _targetmanagerreference)
    (goto _label)))

(fn `UserConstructionScript`)