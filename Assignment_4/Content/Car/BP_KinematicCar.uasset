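; BP_KinematicCar is a player-driven F1 car that moves kinematically, without physics or collision sweeps.
; Throttle and steer inputs ease speed and steering angle toward their maximums, and Tick applies them as forward offset and yaw.
; Yaw ignores speed magnitude, so the car can turn while stationary, and doubles in reverse.
; Tick also feeds both values to the animation Blueprint, while look inputs rotate the spring arm and ToggleCamera swaps chase and in-car cameras.
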(event `self.ReceiveBeginPlay`
  (bind _asf1_car_low_poly_skeleton_anim_blueprint (cast `/Game/Car/F1_car_LowPoly_Skeleton_AnimBlueprint` (`SkeletalMeshComponent.GetAnimInstance` (`self.Car`))))
  (set `self.AnimInstance` _asf1_car_low_poly_skeleton_anim_blueprint))

(event `self.ReceiveTick`
  (params (DeltaSeconds :type "Float (single-precision)"))
  (bind _animinstance (`self.AnimInstance`))
  (bind _currentspeed (`self.CurrentSpeed`))
  (`self.K2_AddActorWorldOffset` (* DeltaSeconds (* (`self.GetActorForwardVector`) _currentspeed)))
  (`self.K2_AddActorWorldRotation` (`KismetMathLibrary.MakeRotator` 0.0 0.0 (* (`GameplayStatics.GetWorldDeltaSeconds`) (`self.CurrentSteeringAngle`) (select `bool` (< _currentspeed 0.0) :`false` 1.0 :`true` 2.0))))
  (set `/Game/Car/F1_car_LowPoly_Skeleton_AnimBlueprint.Speed` (`self.CurrentSpeed`) _animinstance)
  (set `/Game/Car/F1_car_LowPoly_Skeleton_AnimBlueprint.SteeringAngle` (`self.CurrentSteeringAngle`) _animinstance))

(event `InputAxis|Throttle`
  (params (AxisValue :type "Float (single-precision)"))
  (set `self.CurrentSpeed` (`KismetMathLibrary.FInterpTo` (`self.CurrentSpeed`) (* AxisValue (`self.MaxSpeed`)) (`GameplayStatics.GetWorldDeltaSeconds`) 0.1)))

(event `InputAxis|LookRight`
  (params (AxisValue :type "Float (single-precision)"))
  (`SceneComponent.K2_AddRelativeRotation` (`self.SpringArm`) (`KismetMathLibrary.MakeRotator` 0.0 0.0 AxisValue) false false))

(event `InputAxis|LookUp`
  (params (AxisValue :type "Float (single-precision)"))
  (`SceneComponent.K2_AddRelativeRotation` (`self.SpringArm`) (`KismetMathLibrary.MakeRotator` 0.0 AxisValue) false false))

(event `InputAxis|Steer`
  (params (AxisValue :type "Float (single-precision)"))
  (set `self.CurrentSteeringAngle` (`KismetMathLibrary.FInterpTo` (`self.CurrentSteeringAngle`) (* AxisValue (`self.MaxSteeringAngle`)) (`GameplayStatics.GetWorldDeltaSeconds`) 2.0)))

(event `InputAction|ToggleCamera`
  (params (Key :type "Key Structure"))
  (:`Pressed`
    (bind _isa (`/Engine/EditorBlueprintResources/StandardMacros.FlipFlop`)
      (:`A`
        _)
      (:`B`
        _))
    (`ActorComponent.SetActive` (`self.ChaseCamera`) (not _isa) false)
    (`ActorComponent.SetActive` (`self.InCarCamera`) _isa false)))

(fn `UserConstructionScript`)